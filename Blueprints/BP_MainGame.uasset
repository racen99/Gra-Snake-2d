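; Runs a Paper2D Snake game on an XZ grid, spawning the snake, food and border walls, and updating score and HUD.
; Tick, throttled by a Delay, checks self, wall and food hits by exact location equality, then reads gated arrow-key input and moves the snake.
; Body parts follow their predecessor from tail to head, and eating food adds a tail part.
; Death swaps flipbooks and triggers the HUD game-over, with a gated level reload for restarting.
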(event Custom|Spawn%20New%20Snake%20Part
  (params (Spawn%20Location :type Vector) (Is%20Head :type Boolean))
  ;[1 1 1] Spawn New Snake Part
  (bind _returnvalue (Game|SpawnActorfromClass "/Game/Blueprints/BP_SnakeBodyPart.BP_SnakeBodyPart_C" (Math|Transform|MakeTransform Spawn%20Location "0, 0, 0" "1.000000,1.000000,1.000000") "AlwaysSpawn" 0 0))
  (Sprite|SetFlipbook (Variables|/Game/Blueprints/BP_SnakeBodyPart.BP_SnakeBodyPart_C|GetPaperFlipbook _returnvalue) (select Is%20Head "/Game/Flipbooks/skorka1w_Flipbook.skorka1w_Flipbook" "/Game/Flipbooks/skorka1w_Flipbook.skorka1w_Flipbook"))
  (Utilities|Array|Add (Variables|Default|GetSnake%20Parts%20Array) _returnvalue)
  (Variables|/Game/Blueprints/BP_SnakeBodyPart.BP_SnakeBodyPart_C|SetIs%20Head _returnvalue Is%20Head)
  (Transformation|SetActorRotation _returnvalue (Math|Rotator|MakeRotator 0.0 (Utilities|Select :Index (Math|Random|RandomInteger 3) :Option%200 0.0 :Option%201 9e+01 :Option%202 1.8e+02 :Option%203 2.7e+02) 0.0)))

(event Custom|Spawn%20Food
  (bind _x_max (Variables|Default|GetX_Max))
  (bind _z_max (Variables|Default|GetZ_Max))
  (bind _returnvalue (- _x_max 1e+02))
  (bind _returnvalue_2 (- _z_max 1e+02))
  ;[1 1 1] Spawn Food
  (bind _returnvalue_3 (Game|SpawnActorfromClass "/Game/Blueprints/BP_Food.BP_Food_C" (Math|Transform|MakeTransform (Math|Vector|MakeVector (Math|Conversions|ToFloat(Integer) (* (.ReturnValue (Math|Float|Division(WholeandRemainder) (Math|Random|RandomFloatinRange (* _returnvalue -1.0) _returnvalue) 1e+02)) 100)) 0.0 (Math|Conversions|ToFloat(Integer) (* (.ReturnValue (Math|Float|Division(WholeandRemainder) (Math|Random|RandomFloatinRange (* _returnvalue_2 -1.0) _returnvalue_2) 1e+02)) 100))) "0, 0, 0" "1.000000,1.000000,1.000000") "AlwaysSpawn" 0 0))
  (Variables|Default|SetFood%20Actor%20REF _returnvalue_3))

(event Custom|Kill%20Snake
  ;[1 1 1] Kill Snake
  (Variables|Default|SetIs%20Dead true)
  (for (_array_element _array_index) (Variables|Default|GetSnake%20Parts%20Array)
    (Sprite|SetFlipbook (Variables|/Game/Blueprints/BP_SnakeBodyPart.BP_SnakeBodyPart_C|GetPaperFlipbook _array_element) (select (== _array_index 0) "/Game/Flipbooks/Blank_Flipbook.Blank_Flipbook" "/Game/Flipbooks/dead_Flipbook.dead_Flipbook")))
  (Utilities|FlowControl|Delay 0.5)
  (for _array_element_2 (Variables|Default|GetSnake%20Parts%20Array)
    (Sprite|SetFlipbook (Variables|/Game/Blueprints/BP_SnakeBodyPart.BP_SnakeBodyPart_C|GetPaperFlipbook _array_element_2) "/Game/Flipbooks/Blank_Flipbook.Blank_Flipbook")))

(event Custom|Update%20Score
  (params (Value :type Integer))
  ;[1 1 1] Update Score
  (bind _output_get (Variables|Default|SetScore (+ Value (Variables|Default|GetScore))))
  (Default|UpdateScore (Variables|Default|GetHUD%20REF) _output_get)
  (Audio|PlaySound2D "/Game/Music/mario-coin-200bpm-82548.mario-coin-200bpm-82548" 1.0 1.0 0.0 0 0))

(event EventBeginPlay
  ;[1 1 1] Initialize Game
  (|CreateHUDWidget
    (:next
      (|SelectRandomStartDirection)
      (|SetUpdateDelay(SnakeSpeed))
      (|SpawnSnakeHead)
      (|Spawn1stFood)
      (|SpawnWalls))))

(event EventTick
  (params (DeltaSeconds :type Float%20%28single-precision%29))
  (|CheckForDeathCondition1
    (:Is%20Dead
      (|RestartSequence))
    (:Is%20Not%20Dead
      (|Wait
        (:Completed
          (|Sequence1
            (:Do%20First
              (|CheckHeadSelfCollision
                (:Completed
                  (|CheckHeadWallCollision))))
            (:Do%20Second
              (|CheckDeadCondition2
                (:Not%20Dead
                  (|Sequence2
                    (:Do%20First
                      (|CheckHeadFoodCollision
                        (:true
                          (|UpdateGameScore)
                          (|DestroyCurrentFood)
                          (|SpawnSnakeNewPart)
                          (|SpawnNewFood))))
                    (:Do%20Second
                      (|CheckInputs
                        (:Next
                          (|MoveSnake))))))))))))))

(fn ConstructionScript)

(event Custom|Break%20Self%20Collision%20Test%20Loop
  (Utilities|Array|ForEachLoopwithBreak (Variables|Default|GetSnake%20Parts%20Array)) ; enters at Break
)

(event Custom|Break%20Wall%20Collision%20Test%20Loop
  (Utilities|Array|ForEachLoopwithBreak (Variables|Default|GetWall%20Block%20Array)) ; enters at Break
)

(event Input|KeyboardEvents|Up
  (params (Key :type Key%20Structure))
  (:Pressed
    (Utilities|FlowControl|Gate true) ; enters at Open
  )
  (:Released
    (Utilities|FlowControl|Gate true) ; enters at Close
  ))

(event Input|KeyboardEvents|Down
  (params (Key :type Key%20Structure))
  (:Pressed
    (Utilities|FlowControl|Gate true) ; enters at Open
  )
  (:Released
    (Utilities|FlowControl|Gate true) ; enters at Close
  ))

(event Input|KeyboardEvents|Right
  (params (Key :type Key%20Structure))
  (:Pressed
    (Utilities|FlowControl|Gate true) ; enters at Open
  )
  (:Released
    (Utilities|FlowControl|Gate true) ; enters at Close
  ))

(event Input|KeyboardEvents|Left
  (params (Key :type Key%20Structure))
  (:Pressed
    (Utilities|FlowControl|Gate true) ; enters at Open
  )
  (:Released
    (Utilities|FlowControl|Gate true) ; enters at Close
  ))